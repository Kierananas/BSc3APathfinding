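; Grid tile actor for a pathfinding grid, displaying ground type, hover, selection and path state.
; Cursor and click events on its mesh notify BpGrid of the hovered or selected tile.
; SetTileColour reads tile data from BpGrid's map by GridIndex and drives material parameters, with path colour overriding hover brightening.
; Debug events tint open and closed set tiles, and a widget receives the grid and index shortly after BeginPlay.
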(event OnBeginCursorOver(StaticMesh1)
  (params (TouchedComponent :type Primitive%20Component%20Object%20Reference))
  (CallFunction|EventStartOverTile)
  (Default|EventNewTileOvered (Variables|Grid|Getbp_Grid) self))

(event OnEndCursorOver(StaticMesh1)
  (params (TouchedComponent :type Primitive%20Component%20Object%20Reference))
  (Default|EventNewTileOvered (Variables|Grid|Getbp_Grid)))

(event OnClicked(StaticMesh1)
  (params (TouchedComponent :type Primitive%20Component%20Object%20Reference) (ButtonPressed :type Key%20Structure :default "None"))
  (CallFunction|EventSelectTile)
  (Default|EventNewTileSelected (Variables|Grid|Getbp_Grid) self))

(event Custom|Event_SelectTile
  (Variables|Grid|SetbIsSelected true)
  (Grid|SetTileColour))

(event Custom|Event_DeselectTile
  (Variables|Grid|SetbIsSelected false)
  (Grid|SetTileColour))

(event Custom|Event_StartOverTile
  (Variables|Grid|SetbIsOvered true)
  (Grid|SetTileColour))

(event Custom|Event_EndOverTile
  (Variables|Grid|SetbIsOvered false)
  (Grid|SetTileColour))

(event Custom|Event_IsInPath
  (params (Is%20In%20Path :type Boolean))
  (Variables|Default|SetbIsInPath Is%20In%20Path)
  (Grid|SetTileColour))

(event Custom|DebugEvent_OpenSet
  (Rendering|Material|SetVectorParameterValueonMaterials (Variables|Default|GetStaticMesh1) "TileColour" (Math|Conversions|ToVector(LinearColor) "(R=0.000000,G=0.432292,B=0.160589,A=1.000000)")))

(event Custom|DebugEvent_ClosedSet
  (Rendering|Material|SetVectorParameterValueonMaterials (Variables|Default|GetStaticMesh1) "TileColour" (Math|Conversions|ToVector(LinearColor) "(R=0.635417,G=0.029720,B=0.000000,A=1.000000)")))

(event EventBeginPlay
  (Utilities|FlowControl|Delay 0.2)
  (Grid|SetTileColour)
  (CallFunction|SetWidgetVariables))

(fn ConstructionScript)

(fn SetTileColour
  (Utilities|FlowControl|Sequence
    (:then_0
      (switch Utilities|FlowControl|Switch|SwitchonEnum_GroundTypes (.groundtype (Grid|GetTileData))
        (:NewEnumerator0
          (LocalVariables|SetTileColour "(R=1.000000,G=0.839454,B=0.329681,A=1.000000)"))
        (:NewEnumerator1
          (LocalVariables|SetTileColour "(R=1.000000,G=0.770607,B=0.000000,A=1.000000)"))
        (:NewEnumerator2
          (LocalVariables|SetTileColour "(R=1.000000,G=0.221820,B=0.000000,A=1.000000)"))
        (:NewEnumerator3
          (LocalVariables|SetTileColour "(R=1.000000,G=0.024480,B=0.000000,A=1.000000)"))
        (:NewEnumerator4
          (LocalVariables|SetTileColour "(R=0.026042,G=0.026042,B=0.026042,A=1.000000)"))))
    (:then_1
      (if (Variables|Grid|GetbIsSelected)
        (Rendering|Material|SetScalarParameterValueonMaterials (Variables|Default|GetStaticMesh1) "bIsSelected" 1.0)
        (else
          (Rendering|Material|SetScalarParameterValueonMaterials (Variables|Default|GetStaticMesh1) "bIsSelected" 0.0))))
    (:then_2
      (if (Variables|Grid|GetbIsOvered)
        (LocalVariables|SettileColour (Math|Conversions|ToLinearColor(Vector) (* (Math|Conversions|ToVector(LinearColor) (LocalVariables|GettileColour)) 3.0)))))
    (:then_3
      (if (Variables|Default|GetbIsInPath)
        (LocalVariables|SetTileColour "(R=0.063430,G=0.000000,B=1.000000,A=1.000000)")))
    (:then_4
      (Rendering|Material|SetVectorParameterValueonMaterials (Variables|Default|GetStaticMesh1) "TileColour" (Math|Conversions|ToVector(LinearColor) (LocalVariables|GettileColour))))))

(fn GetTileData
  (return (.Value (Utilities|Map|Find (Variables|/Game/Blueprints/Grid/BP_Grid.BP_Grid_C|Getstruct_Tiles (Variables|Grid|Getbp_Grid)) (Variables|Grid|GetgridIndex)))))

(fn SetTileSize
  (bind _bp_grid (Variables|Grid|Getbp_Grid))
  (bind _staticmesh1 (Variables|Default|GetStaticMesh1))
  (bind _returnvalue (Transformation|GetWorldScale _staticmesh1))
  (bind _tilesize (Variables|/Game/Blueprints/Grid/BP_Grid.BP_Grid_C|GetTileSize _bp_grid))
  (bind _returnvalue_2 (/ _tilesize 5e+01))
  (bind _returnvalue_3 (* _returnvalue _returnvalue_2))
  (Transformation|SetWorldScale3D _staticmesh1 (Math|Vector|MakeVector (.x _returnvalue_3) (.y _returnvalue_3) 1.0)))

(fn SetWidgetVariables
  (bind _widget (Variables|Default|GetWidget))
  (bind _returnvalue (UserInterface|GetUserWidgetObject _widget))
  (bind _asw_grid_tile (Utilities|Casting|CastToW_GridTile _returnvalue))
  (Variables|/Game/Blueprints/Grid/W_GridTile.W_GridTile_C|Setgrid _asw_grid_tile (Variables|Grid|Getbp_Grid))
  (Variables|/Game/Blueprints/Grid/W_GridTile.W_GridTile_C|SetgridIndex _asw_grid_tile (Variables|Grid|GetgridIndex)))