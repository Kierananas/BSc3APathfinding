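; HUD Blueprint that draws an RTS-style marquee selection box on screen.
; Input start, hold and release events record the clicked and current mouse positions and toggle a drawing flag; a drag begins only while SelectedUnits is empty.
; While that flag is set, DrawHUD calls the marquee event, which renders a translucent light-blue rectangle and two corner points.
; The file only draws the box, without selecting units.
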(event Custom|Event_DrawMarquee
  (bind _clickedlocation (Variables|MarqueeVariables|GetClickedLocation))
  (bind _holdinglocation (Variables|MarqueeVariables|GetHoldingLocation))
  (bind _clickedlocation_2 (Variables|MarqueeVariables|GetClickedLocation))
  (bind _holdinglocation_2 (Variables|MarqueeVariables|GetHoldingLocation))
  (bind _clickedlocation_3 (Variables|MarqueeVariables|GetClickedLocation))
  (bind (_x _y) (Math|Vector2D|BreakVector2D _holdinglocation))
  (bind (_x_2 _y_2) (Math|Vector2D|BreakVector2D _clickedlocation_2))
  (bind _returnvalue (- _holdinglocation_2 _clickedlocation_3))
  (bind (_x_3 _y_3) (Math|Vector2D|BreakVector2D _clickedlocation))
  (bind (_x_4 _y_4) (Math|Vector2D|BreakVector2D _returnvalue))
  (HUD|DrawRect "(R=0,G=0,B=0,A=1)" _x_3 _y_3 1.0 1.0)
  (HUD|DrawRect "(R=0,G=0,B=0,A=1)" _x _y 1.0 1.0)
  (HUD|DrawRect "(R=0.463542,G=0.892201,B=1.000000,A=0.600000)" _x_2 _y_2 _x_4 _y_4))

(event EventBeginPlay
  (Variables|Referrences|SetControllerRef (.AsBP%20Player%20Controller (Utilities|Casting|CastToBP_PlayerController (Game|GetPlayerController 0)))))

(event EventOnInputStart
  (bind _controllerref (Variables|Referrences|GetControllerRef))
  (bind (_locationx _locationy) (Game|Player|GetMousePosition _controllerref))
  (if (not (>= (Utilities|Array|LastIndex (Variables|Units|GetSelectedUnits)) 0))
    (bind _output_get (Variables|MarqueeVariables|SetClickedLocation (Math|Vector2D|MakeVector2D _locationx _locationy)))
    (Variables|MarqueeVariables|SetHoldingLocation _output_get)
    (Variables|Boolean|SetIsDrawing true)))

(event EventOnInputRelease
  (params (HoldTime :type Float%20%28single-precision%29))
  (Variables|Boolean|SetIsDrawing false))

(event EventDrawHUD
  (params (SizeX :type Integer) (SizeY :type Integer))
  (if (Variables|Boolean|GetIsDrawing)
    (Utilities|FlowControl|Sequence
      (:then_0
        (CallFunction|EventDrawMarquee)))))

(event EventOnInputHold
  (bind _controllerref (Variables|Referrences|GetControllerRef))
  (bind (_locationx _locationy) (Game|Player|GetMousePosition _controllerref))
  (Variables|MarqueeVariables|SetHoldingLocation (Math|Vector2D|MakeVector2D _locationx _locationy)))

(fn ConstructionScript)