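; Player controller for an RTS-style game that tracks the selected unit, deselects the previous one and passes new paths to it to follow.
; Outside building mode, left mouse press, hold time and release drive marquee selection on the RTS_MarqueeSelectionBP HUD.
; R toggles obstacle visibility and T toggles slow motion.
; An AI move-to-cursor order with destination decal for multiple units is present but unconnected.
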(event Custom|Event_NewUnitSelected
  (params (Unit :type BP%20Unit%20Object%20Reference))
  (Utilities|IsValid (Variables|UnitControl|GetselectedUnit)
    (:Is%20Valid
      (Default|EventDeselected (Variables|UnitControl|GetselectedUnit)))
    (:Is%20Not%20Valid
      _))
  (Variables|UnitControl|SetselectedUnit Unit))

(event Custom|Event_NewPathAvailable
  (params (path :type Array%20of%20Vector%202D%20Structures))
  (Utilities|IsValid (Variables|UnitControl|GetselectedUnit)
    (:Is%20Valid
      (Default|EventMoveAlongthePath (Variables|UnitControl|GetselectedUnit) path))))

(event Custom|UpdateSelection
  (if (Variables|Boolean|GetIsHoldingInput)
    (Variables|MarqueeVariables|SetHoldingTime (+ (Variables|MarqueeVariables|GetHoldingTime) (Variables|MarqueeVariables|GetDeltaTime)))
    (Class|RTSMarqueeSelectionIF|OnInputHold(Message) (Variables|Referrences|GetMarqueeRef))))

(event EventBeginPlay
  (bind _asrts_marquee_selection_bp (Utilities|Casting|CastToRTS_MarqueeSelectionBP (HUD|GetHUD)))
  (Variables|Referrences|SetMarqueeRef _asrts_marquee_selection_bp))

(event EventTick
  (params (DeltaSeconds :type Float%20%28single-precision%29))
  (Variables|MarqueeVariables|SetDeltaTime DeltaSeconds)
  (if (Variables|Boolean|GetIsHoldingInput)
    (CallFunction|UpdateSelection)))

(event Input|KeyboardEvents|R
  (params (Key :type Key%20Structure :default "None"))
  (:Pressed
    (Utilities|FlowControl|FlipFlop
      (:A
        (bind _outactors (Actor|GetAllActorsOfClass "/Game/Blueprints/Grid/BP_Base_Obstacle.BP_Base_Obstacle_C"))
        (for _array_element _outactors
          (Rendering|SetActorHiddenInGame _array_element true)))
      (:B
        (bind _outactors_2 (Actor|GetAllActorsOfClass "/Game/Blueprints/Grid/BP_Base_Obstacle.BP_Base_Obstacle_C"))
        (for _array_element_2 _outactors_2
          (Rendering|SetActorHiddenInGame _array_element_2 false))))))

(event Input|KeyboardEvents|T
  (params (Key :type Key%20Structure :default "None"))
  (:Pressed
    (Utilities|FlowControl|FlipFlop
      (:A
        (Utilities|Time|SetGlobalTimeDilation 0.1))
      (:B
        (Utilities|Time|SetGlobalTimeDilation 1.0)))))

(event Input|MouseEvents|LeftMouseButton
  (params (Key :type Key%20Structure :default "None"))
  (bind _selectedunitsvariable (Variables|UnitControl|GetSelectedUnitsVariable))
  (bind _isbuildingmodeactive (Variables|Boolean|GetIsBuildingModeActive))
  (:Pressed
    (if _isbuildingmodeactive
      (UnitControl|SetSelectedUnits _selectedunitsvariable)
      (for _array_element _selectedunitsvariable
        (Variables|UnitControl|SetselectedUnit 0))
      (else
        (Class|RTSMarqueeSelectionIF|OnInputStart(Message) (Variables|Referrences|GetMarqueeRef))
        (Variables|MarqueeVariables|SetHoldingTime 0.0)
        (Variables|Boolean|SetIsHoldingInput true))))
  (:Released
    (if (not _isbuildingmodeactive)
      (Class|RTSMarqueeSelectionIF|OnInputRelease(Message) (Variables|Referrences|GetMarqueeRef) (Variables|MarqueeVariables|GetHoldingTime))
      (Variables|Boolean|SetIsHoldingInput false))))

(event Input|MouseEvents|RightMouseButton
  (params (Key :type Key%20Structure :default "None"))
  ;[1 1 1] Comment
)

(fn ConstructionScript)

(fn SetSelectedUnits
  (params (SelectedUnits :type Array%20of%20BP%20Unit%20Object%20References))
  (Variables|UnitControl|SetSelectedUnitsVariable SelectedUnits)
  (if (>= (Utilities|Array|LastIndex (Variables|UnitControl|GetSelectedUnitsVariable)) 0)
    (Variables|Boolean|SetIsUnitSelected true)))